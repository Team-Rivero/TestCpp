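; Security camera actor that turns to face the nearest Pawn within its Radius.
; Each Tick it stores the nearest Pawn and, if valid, snaps its whole rotation to look at that Pawn's location, with no interpolation.
; It also runs a forward Visibility line trace with per-frame debug drawing, but the result is unused, so line of sight does not affect tracking.
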(event `self.ReceiveTick`
  (params (DeltaSeconds :type "Float (single-precision)"))
  (bind _returnvalue (`self.K2_GetActorLocation`))
  (`KismetSystemLibrary.LineTraceSingle` :`Start` _returnvalue :`End` (+ _returnvalue (* (`self.GetActorForwardVector`) 1000.0)) :`TraceChannel` "TraceTypeQuery1" :`DrawDebugType` "ForOneFrame")
  (bind _returnvalue_2 (`BlueprintFunctionLibraryA.GetNearestActorOfClass` "/Script/Engine.Pawn" (`self.K2_GetActorLocation`) (`self.Radius`)))
  (bind _output_get (set `self.NearestPawn` _returnvalue_2))
  (`/Engine/EditorBlueprintResources/StandardMacros.IsValid` _output_get
    (:`Is Valid`
      (`self.K2_SetActorRotation` (`KismetMathLibrary.FindLookAtRotation` (`self.K2_GetActorLocation`) (`self.K2_GetActorLocation` (`self.NearestPawn`)))))))

(fn `UserConstructionScript`)